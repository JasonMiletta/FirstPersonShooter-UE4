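; Base enemy Blueprint that handles health, contact damage and weapon pickup drops.
; AnyDamage subtracts Health unless the causer is another Parent_Enemy, then at zero or below rolls ItemDropChance as a percentage and destroys the actor.
; A successful roll spawns a randomly picked AutoGun or TriShot pickup at the enemy's location.
; Hit applies Damage to the other actor and adds an impulse along the negated hit normal.
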(event `self.ReceiveAnyDamage`
  (params (Damage :type "Float (single-precision)") (DamageType :type "DamageType Object Reference") (InstigatedBy :type "Controller Object Reference") (DamageCauser :type "Actor Object Reference"))
  ;[1 1 1] HP Handling
  (if (not (`KismetMathLibrary.ClassIsChildOf` (`GameplayStatics.GetObjectClass` DamageCauser) "Parent_Enemy_C"))
    (bind _output_get (set `self.Health` (- (`self.Health`) Damage))))
  (if (>= 0.0 _output_get)
    ;[1 1 1] Drop Items
    (bind _dropitem (`self.Should Drop Item`))
    (if _dropitem
      (bind _item (`self.Pick Item Drop`))
      (`|SpawnActorFromClass` _item (`KismetMathLibrary.MakeTransform` (`self.K2_GetActorLocation`)) true))
    (`self.K2_DestroyActor`)))

(event `self.ReceiveHit`
  (params (MyComp :type "PrimitiveComponent Object Reference") (Other :type "Actor Object Reference") (OtherComp :type "PrimitiveComponent Object Reference") (bSelfMoved :type Boolean) (HitLocation :type "Object.Vector Structure") (HitNormal :type "Object.Vector Structure") (NormalImpulse :type "Object.Vector Structure") (Hit :type "EngineTypes.HitResult Structure (by ref)"))
  ;[1 1 1] Damage Handling
  (`GameplayStatics.ApplyDamage` Other (`self.Damage`) (`self.GetController`) self)
  (`CharacterMovementComponent.AddImpulse` (`KismetMathLibrary.NegateVector` HitNormal)))

(fn `Pick Item Drop`
  (returns (Item :type "/Game/Blueprints/WeaponPickups/BP_Parent_Gun_Pickup Class Reference"))
  (switch `int` (`KismetMathLibrary.RandomInteger` 2)
    (:`Default`
      (set `self.Item` "/Game/Blueprints/WeaponPickups/WeaponPickup_TriShot.WeaponPickup_TriShot_C"))
    (:`0`
      (set `self.Item` "/Game/Blueprints/WeaponPickups/WeaponPickup_AutoGun.WeaponPickup_AutoGun_C"))
    (:`1`
      (set `self.Item` "/Game/Blueprints/WeaponPickups/WeaponPickup_TriShot.WeaponPickup_TriShot_C")))
  (return (`self.Item`)))

(fn `Should Drop Item`
  (returns (dropItem :type Boolean))
  (return (> (`self.ItemDropChance`) (* (`KismetMathLibrary.RandomFloat`) 100.0))))

(fn `UserConstructionScript`)