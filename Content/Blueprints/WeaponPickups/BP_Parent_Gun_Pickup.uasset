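; Parent weapon pickup that switches the player to its weapon type when walked over.
; BeginPlay sets a default type and "Basic Gun" label, then plays a timeline that adds vertical offsets to move the actor.
; Overlap by the player pawn destroys the pickup, then calls ChangeWeapon on MyCharacter.
; Tick turns the name text toward the player, using a look-at rotation applied as relative rotation.
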(event `self.ReceiveBeginPlay`
  (set `self.Weapon Type` "NewEnumerator0")
  (`TextRenderComponent.SetText` (`self.Name`) "Basic Gun")
  (bind (_direction _z_vector) (`Timeline|Timeline_0`)
    (:`Update`
      (`self.K2_AddActorLocalOffset` (* _z_vector 0.5)))))

(event `self.ReceiveActorBeginOverlap`
  (params (OtherActor :type "Actor Object Reference"))
  ;[1 1 1] Player Picked Up Weapon
  (if (== OtherActor (`GameplayStatics.GetPlayerPawn` 0))
    (`self.K2_DestroyActor`)
    (bind _asmy_character (cast `/Game/Blueprints/MyCharacter` OtherActor))
    (`/Game/Blueprints/MyCharacter.ChangeWeapon` _asmy_character (`self.Weapon Type`))))

(event `self.ReceiveTick`
  (params (DeltaSeconds :type "Float (single-precision)"))
  (bind _returnvalue (`GameplayStatics.GetPlayerCharacter` 0))
  (bind _name (`self.Name`))
  ;[1 1 1] Rotate Name To Face Player
  (if (`KismetSystemLibrary.IsValid` _returnvalue)
    (`SceneComponent.K2_SetRelativeRotation` _name (`KismetMathLibrary.FindLookAtRotation` (`SceneComponent.K2_GetComponentLocation` _name) (`self.K2_GetActorLocation` _returnvalue)) false)))

(fn `UserConstructionScript`)